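; BP_MagicDoor is a door that swings open and closed in response to a separate Trigger interactable.
; On BeginPlay it validates Trigger and its BPC_Interaction component, then binds to that component's interact event.
; The event's On state plays or reverses the DoorAnimation timeline, which drives the AnchorHinge relative yaw through a quarter turn.
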(event `self.ReceiveBeginPlay`
  ;[0 0 0] Checks that Trigger is set
  (bind _trigger (`self.Trigger`)
    (:`then`
      (bind _returnvalue (`self.GetComponentByClass` _trigger "/Game/Blueprints/Game/Components/BPC_Interaction.BPC_Interaction_C"))
      ;[0 0 0] Checks that Trigger has a BPC_Interation
      (`/Engine/EditorBlueprintResources/StandardMacros.IsValid` _returnvalue
        (:`Is Valid`
          (add `/Game/Blueprints/Game/Components/BPC_Interaction.OnInteract` _returnvalue (delegate `OnInteract_Event`)))))
    (:`else`)))

(event `OnInteract_Event`
  (params (On :type Boolean))
  (if On
    (`self.OpenDoor`)
    (else
      (`self.Close Door`))))

(event `OpenDoor`
  (bind (_direction _doormovement) (`Timeline|DoorAnimation` :!label _label)
    (:`Update`
      (`SceneComponent.K2_SetRelativeRotation` (`self.Anchor_Hinge`) (`KismetMathLibrary.MakeRotator` 0.0 0.0 (* _doormovement 90.0)) false false))))

(event `Close Door`
  (goto _label :!via `Reverse`))

(fn `UserConstructionScript`
  (`parent.UserConstructionScript`))