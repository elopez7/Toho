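; BP_ConduitCrystal is an interactable crystal whose radius grows when switched on and shrinks when switched off.
; It binds to its interaction component's OnInteract event, which plays or reverses the ChangeRadius timeline.
; The timeline scales the Cylinder's X and Y from its Radius curve times RadiusScalar plus InteractionRadius, keeping height fixed.
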(event `self.ReceiveBeginPlay`
  (add `/Game/Blueprints/Game/Components/BPC_Interaction.OnInteract` (`self.BPC_Interaction`) (delegate `OnInteract_Event`)))

(event `OnInteract_Event`
  (params (On :type Boolean))
  (if On
    (`self.IncreaseRadius`)
    (else
      (`self.DecreaseRadius`))))

(event `IncreaseRadius`
  (bind (_direction _radius) (`Timeline|ChangeRadius` :!label _label)
    (:`Update`
      (bind _returnvalue (+ (* _radius (`self.RadiusScalar`)) (`self.InteractionRadius`)))
      (`SceneComponent.SetRelativeScale3D` (`self.Cylinder`) (`KismetMathLibrary.MakeVector` _returnvalue _returnvalue 1.0)))))

(event `DecreaseRadius`
  (goto _label :!via `Reverse`))

(fn `UserConstructionScript`
  (`parent.UserConstructionScript`))