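; Health component that tracks an actor's current health and death state.
; CurrentHealth starts at MaxHealth on BeginPlay.
; ReceiveDamage subtracts damage, clamps the result between zero and MaxHealth, and sets IsDead when health reaches zero.
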(event `self.ReceiveBeginPlay`
  (set `self.CurrentHealth` (`self.MaxHealth`)))

(fn `ReceiveDamage`
  (params (DamageAmount :type "Float (double-precision)"))
  (bind _output_get (set `self.CurrentHealth` (`KismetMathLibrary.FClamp` (- (`self.CurrentHealth`) DamageAmount) 0.0 (`self.MaxHealth`))))
  (if (<= _output_get 0.0)
    (set `self.IsDead` true)))