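; BPC_Magic is an actor component that tracks a magic point pool for spellcasting.
; BeginPlay fills CurrentMP to MaxMP.
; CastMagic compares a cost to CurrentMP, then either prints a warning and clears CanCastMagic, or deducts the clamped cost and sets CanCastMagic to true.
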(event `self.ReceiveBeginPlay`
  (set `self.CurrentMP` (`self.MaxMP`)))

(fn `CastMagic`
  (params (MPCost :type "Float (double-precision)"))
  (if (> MPCost (`self.CurrentMP`))
    (`KismetSystemLibrary.PrintString` "Not enough magic points")
    (set `self.CanCastMagic` false)
    (else
      (set `self.CurrentMP` (`KismetMathLibrary.FClamp` (- (`self.CurrentMP`) MPCost) 0.0 (`self.MaxMP`)))
      (set `self.CanCastMagic` true))))